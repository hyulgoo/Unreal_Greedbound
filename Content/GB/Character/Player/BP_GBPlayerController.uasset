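; Player controller Blueprint that sets up the player's UI and input settings when InitializePlayerUI fires.
; It creates WBP_PrimaryLayout, adds it to the viewport and registers it with GBUISubsystem, which then sets the HUD widget using the Ability System Component.
; It also registers IMC_Gameplay with Enhanced Input user settings, which does not itself add the mapping context.
; BeginPlay, Tick and Possess are empty.
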(event `self.ReceiveBeginPlay`)

(event `self.ReceivePossess`
  (params (PossessedPawn :type "Pawn Object Reference")))

(event `self.InitializePlayerUI`
  (`|ExecutionSequence`
    (:`then_0`
      (bind _returnvalue (`|CreateWidget` "/Game/GB/UI/InGame/Widgets/WBP_PrimaryLayout.WBP_PrimaryLayout_C" self))
      (`UserWidget.AddToViewport` _returnvalue 0)
      (`GBUISubsystem.RegisterCreatedPrimaryLayoutWidget` (subsystem `GBUISubsystem`) _returnvalue)
      (bind _returnvalue_2 (`self.GetAbilitySystemComponent` self))
      (`GBUISubsystem.SetHUDWidget` (subsystem `GBUISubsystem`) _returnvalue_2))
    (:`then_1`
      (`EnhancedInputUserSettings.RegisterInputMappingContext` (`EnhancedInputSubsystemInterface.GetUserSettings` (subsystem `EnhancedInputLocalPlayerSubsystem`)) "/Game/GB/Input/InputMappingContexts/IMC_Gameplay.IMC_Gameplay"))))

(fn `UserConstructionScript`)